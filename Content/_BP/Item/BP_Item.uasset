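; BP_Item is a pickup item actor that the player collects by touching it.
; When its Sphere overlaps an actor tagged Player, it passes its ItemType to that actor's PickUpMessage and runs PickItem.
; PickItem plays a 2D pickup sound, calls CallDestroyItem with the type and destroys the actor.
; The construction script sets ItemType to the first enum entry.
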(event `self.Sphere.OnComponentBeginOverlap`
  (params (OverlappedComponent :type "PrimitiveComponent Object Reference") (OtherActor :type "Actor Object Reference") (OtherComp :type "PrimitiveComponent Object Reference") (OtherBodyIndex :type Integer) (bFromSweep :type Boolean) (SweepResult :type "HitResult Structure (by ref)"))
  (if (`self.ActorHasTag` OtherActor "Player")
    (message `/Game/_BP/BPI_PickUp.PickUp` OtherActor (`self.ItemType`))
    (`self.PickItem`)))

(event `PickItem`
  (`GameplayStatics.PlaySound2D` "/Game/sound/EffectSound/Item_Get.Item_Get" 1.0 1.0 0.0 null null)
  (`self.Destroy item` (`self.ItemType`))
  (`self.K2_DestroyActor`))

(fn `UserConstructionScript`
  (set `self.ItemType` "NewEnumerator0"))