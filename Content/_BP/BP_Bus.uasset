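; BP_Bus is a drivable bus moved and steered through Enhanced Input actions.
; IA_BusMove applies a swept local offset built from the negated actor forward vector, and IA_BusTurn adds yaw scaled by TurnSpeed, neither using delta time.
; An unconnected debug loop, which never runs, fans visibility line traces using a light's cone angle and attenuation radius.
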(event `EnhancedInput|/Game/Input/IA_BusMove`
  (params (ActionValue :type "Float (double-precision)") (ElapsedSeconds :type "Float (double-precision)") (TriggeredSeconds :type "Float (double-precision)") (InputAction :type "InputAction Object Reference" :default "/Game/Input/IA_BusMove.IA_BusMove"))
  (:`Triggered`
    (`self.K2_AddActorLocalOffset` (* (* ActionValue (`self.GetActorForwardVector`) -1.0) 50.0) true)))

(event `EnhancedInput|/Game/Input/IA_BusTurn`
  (params (ActionValue :type "Float (double-precision)") (ElapsedSeconds :type "Float (double-precision)") (TriggeredSeconds :type "Float (double-precision)") (InputAction :type "InputAction Object Reference" :default "/Game/Input/IA_BusTurn.IA_BusTurn"))
  (:`Triggered`
    (`self.K2_SetActorRotation` (`KismetMathLibrary.MakeRotator` 0.0 0.0 (+ (* (`self.Turn Speed`) ActionValue) (.yaw (`self.K2_GetActorRotation`)))))))

(event `self.ReceiveTick`
  (params (DeltaSeconds :type "Float (single-precision)")))

(fn `UserConstructionScript`)