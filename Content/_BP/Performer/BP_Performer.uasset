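; BP_Performer is a performer actor that plays music quietly and gets a timed volume boost with an aura when exposed to light.
; ExposedLight applies the aura overlay material, raises the sound's volume multiplier and sets a timer for TurnDownVolume, which lowers volume and clears the overlay.
; Tick feeds the timer's remaining fraction to a widget component progress bar.
; Q and E keys manually trigger the boost and reset, with debug prints.
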(event `self.ReceiveBeginPlay`
  (`self.Start Music` null)
  (bind _aswb_volume_up_progress_bar (cast `/Game/UI/WB_VolumeUpProgressBar` (`WidgetComponent.GetWidget` (`self.VolumeUpTimeProgressBar`))))
  (set `self.Volume Up Progress Bar Ref` _aswb_volume_up_progress_bar))

(event `self.ReceiveTick`
  (params (DeltaSeconds :type "Float (single-precision)"))
  (bind _remainingtime (`self.GetRemainingVolumeUpTime`))
  (set `/Game/UI/WB_VolumeUpProgressBar.ProgressPercent` (/ _remainingtime (`self.MaxVolumeUpTime`)) (`self.Volume Up Progress Bar Ref`)))

(event `Key|Q`
  (params (Key :type "Key Structure"))
  (:`Pressed`
    (`self.TurnUpVolume`)
    (`KismetSystemLibrary.PrintString` "BP_Performer > Keyboard E > VolumeUp")
    (`KismetSystemLibrary.PrintString` "Hello")
    (`self.ExposedLight`)))

(event `Key|E`
  (params (Key :type "Key Structure"))
  (:`Pressed`
    (`self.TurnDownVolume`)
    (`KismetSystemLibrary.PrintString` "BP_Performer > Keyboard E > VolumeDown")))

(fn `ExposedLight`
  (`MeshComponent.SetOverlayMaterial` (`self.SkeletalMesh`) "/Game/_Assets/Aura/Aura_grate.Aura_grate")
  (`self.TurnUpVolume`)
  (bind _returnvalue (`KismetSystemLibrary.K2_SetTimer` null "TurnDownVolume" (`self.MaxVolumeUpTime`)))
  (set `self.VolumeUpTimerHandle` _returnvalue))

(fn `GetRemainingVolumeUpTime`
  (returns (RemainingTime :type "Float (double-precision)"))
  (if (`KismetSystemLibrary.K2_IsTimerActiveHandle` (`self.VolumeUpTimerHandle`))
    (return (`KismetSystemLibrary.K2_GetTimerRemainingTimeHandle` (`self.VolumeUpTimerHandle`)))
    (else
      (return 0.0))))

(fn `Start Music`
  (params (SoundBase :type "SoundBase Object Reference"))
  (`AudioComponent.Play` (`self.PerformSound`) 0.0)
  (`self.TurnDownVolume`))

(fn `TurnDownVolume`
  (`AudioComponent.SetVolumeMultiplier` (`self.PerformSound`) (`self.VolumeDownScale`))
  (`MeshComponent.SetOverlayMaterial` (`self.SkeletalMesh`) null))

(fn `TurnUpVolume`
  (`AudioComponent.SetVolumeMultiplier` (`self.PerformSound`) (`self.VolumeUpScale`)))

(fn `UserConstructionScript`)